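; Door actor that applies a solid material and builds an info text from its first actor tag on BeginPlay.
; The UpdateMaterial event sets the first material slot of every static mesh component to the given material, starting with M_Solid.
; InfoText joins "This is" and the tag with no space between them.
; An unconnected copy of the material loop never runs.
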(event `self.ReceiveBeginPlay`
  (bind _tags (`self.Tags`))
  (`self.UpdateMaterial` "/Game/Materials/M_Solid.M_Solid")
  (if (`KismetArrayLibrary.Array_IsValidIndex` _tags)
    (set `self.Info Text` (`KismetSystemLibrary.MakeLiteralText` (`KismetTextLibrary.Conv_StringToText` (`KismetStringLibrary.Concat_StrStr` "This is " (`KismetStringLibrary.Conv_NameToString` (`|GetArrayItem` _tags))))))))

(event `UpdateMaterial`
  (params (`New Material` :type "Material Object Reference"))
  (for _array_element (`self.K2_GetComponentsByClass` "/Script/Engine.StaticMeshComponent")
    (`PrimitiveComponent.SetMaterial` _array_element 0 `New Material`)))

(fn `UserConstructionScript`)