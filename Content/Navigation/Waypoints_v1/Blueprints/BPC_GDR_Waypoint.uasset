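; Actor component that draws a waypoint trail of cylinder spline meshes along the navigation path from its owner to a goal location.
; The server finds the path, then owner events build the spline and meshes on a spawned BP_WaypointManager, since components cannot host components.
; A looping timer rebuilds the trail as the owner moves and clears it near the goal.
; A retriggerable delay removes it after its lifetime.
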(event `Svr_getPath`
  (params (TargetLocation :type "Vector Structure"))
  (`self.GetPath` TargetLocation))

(event `GetPath`
  (params (TargetLocation :type "Vector Structure"))
  (bind _returnvalue (`NavigationSystemV1.FindPathToLocationSynchronously` (`Actor.K2_GetActorLocation` (`self.GetOwner`)) TargetLocation null null))
  (bind _pathpoints (`NavigationPath.PathPoints` _returnvalue))
  (if (and (`NavigationPath.IsValid` _returnvalue) (> (`KismetArrayLibrary.Array_Length` _pathpoints) 0))
    (`self.OwnerCreateWaypoint` _pathpoints)
    (else
      (`self.OwnerResetDelay`))))

(event `OwnerCreateWaypoint`
  (params (Path :type "Array of Vector Structure"))
  (bind _returnvalue (`KismetMathLibrary.MakeVector2D` 0.5 0.5))
  (bind _spline_component (`self.Spline Component`))
  (bind _spline_component_2 (`self.Spline Component`))
  (bind _spline_component_3 (`self.Spline Component`))
  (bind _waypoint_manager (`self.Waypoint Manager`))
  (bind _spline_component_4 (`self.Spline Component`))
  (bind _waypointtimerhandle (`self.WaypointTimerHandle`))
  (bind _output_get (set `self.Path` Path))
  (set `self.WaypointStartLocation` (`|GetArrayItem` _output_get))
  (`/Game/Navigation/Waypoints_v1/Blueprints/BP_WaypointManager.RemoveWaypoint` (`self.Waypoint Manager`))
  (for (_array_element _array_index) (`self.Path`)
    (`SplineComponent.AddSplinePointAtIndex` _spline_component (+ _array_element (`KismetMathLibrary.MakeVector` 0.0 0.0 (`self.Z_Offset`))) _array_index "World" false)
    (`SplineComponent.SetSplinePointType` _spline_component _array_index "Constant" false))
  (`SplineComponent.UpdateSpline` (`self.Spline Component`))
  (for _index (range (`KismetArrayLibrary.Array_LastIndex` (`self.Path`)))
    (bind _returnvalue_2 (`|AddComponentByClass` :`self` (`self.Waypoint Manager`) :`Class` "/Script/Engine.SplineMeshComponent" :`bManualAttachment` true))
    (`KismetArrayLibrary.Array_Add` (`/Game/Navigation/Waypoints_v1/Blueprints/BP_WaypointManager.SplineMeshes` (`self.Waypoint Manager`)) _returnvalue_2)
    (`SceneComponent.SetMobility` _returnvalue_2 "Movable")
    (`StaticMeshComponent.SetStaticMesh` _returnvalue_2 "/Game/Navigation/Waypoints_v1/Mesh/SM_SplineCylinder.SM_SplineCylinder")
    (bind _returnvalue_3 (+ _index 1))
    (`SplineMeshComponent.SetStartAndEnd` _returnvalue_2 (`SplineComponent.GetLocationAtSplinePoint` _spline_component_3 _index "World") (`SplineComponent.GetTangentAtSplinePoint` _spline_component_3 _index "World") (`SplineComponent.GetLocationAtSplinePoint` _spline_component_2 _returnvalue_3 "World") (`SplineComponent.GetTangentAtSplinePoint` _spline_component_2 _returnvalue_3 "World") false)
    (`SplineMeshComponent.SetStartScale` _returnvalue_2 _returnvalue false)
    (`SplineMeshComponent.SetEndScale` _returnvalue_2 _returnvalue true))
  (if (not (`KismetSystemLibrary.K2_IsValidTimerHandle` (`self.WaypointTimerHandle`)))
    (bind _returnvalue_4 (`KismetSystemLibrary.K2_SetTimer` null "WaypointTimer" (`self.UpdateInterval`) true))
    (set `self.WaypointTimerHandle` _returnvalue_4))
  ;[1 1 1] Removes Spline
  (`KismetSystemLibrary.RetriggerableDelay` (`self.SplineLifetime`) :!label _label)
  (`/Engine/EditorBlueprintResources/StandardMacros.IsValid` _waypoint_manager :!label _label_2
    (:`Is Valid`
      (`/Game/Navigation/Waypoints_v1/Blueprints/BP_WaypointManager.RemoveWaypoint` _waypoint_manager))
    (:`Is Not Valid`
      _))
  (`/Engine/EditorBlueprintResources/StandardMacros.IsValid` _spline_component_4
    (:`Is Valid`
      (`SplineComponent.ClearSplinePoints` _spline_component_4 true))
    (:`Is Not Valid`
      _))
  (if (`KismetSystemLibrary.K2_IsValidTimerHandle` _waypointtimerhandle)
    (`KismetSystemLibrary.K2_ClearAndInvalidateTimerHandle` _waypointtimerhandle)))

(event `CreateWaypoint`
  (params (GoalDistance :type "Float (double-precision)") (GoalLocation :type "Vector Structure") (UpdateInterval :type "Float (double-precision)") (Z_Offset :type "Float (double-precision)") (UpdateDistance :type "Float (double-precision)") (SplineLifetime :type "Float (double-precision)"))
  (bind _targetlocation (`self.TargetLocation`))
  (set `self.GoalDistance` GoalDistance)
  (set `self.TargetLocation` GoalLocation)
  (set `self.UpdateInterval` UpdateInterval)
  (set `self.Z_Offset` Z_Offset)
  (set `self.UpdateDistance` UpdateDistance)
  (set `self.SplineLifetime` SplineLifetime)
  ;[0 0 0] We cannot add components to another component, so we create an Actor which we can add and remove components from.
  (`/Engine/EditorBlueprintResources/StandardMacros.IsValid` (`self.Waypoint Manager`)
    (:`Is Valid`
      _)
    (:`Is Not Valid`
      (bind _returnvalue (`|SpawnActorFromClass` "/Game/Navigation/Waypoints_v1/Blueprints/BP_WaypointManager.BP_WaypointManager_C" (`KismetMathLibrary.MakeTransform` (0.0 0.0 0.0)) "AlwaysSpawn" "MultiplyWithRoot" null null))
      (set `self.Waypoint Manager` _returnvalue)))
  (`/Engine/EditorBlueprintResources/StandardMacros.IsValid` (`self.Spline Component`)
    (:`Is Valid`
      (`SplineComponent.ClearSplinePoints` (`self.Spline Component`) true))
    (:`Is Not Valid`
      (bind _returnvalue_2 (`|AddComponentByClass` :`self` (`self.Waypoint Manager`) :`Class` "/Script/Engine.SplineComponent"))
      (set `self.Spline Component` _returnvalue_2)))
  (`KismetArrayLibrary.Array_Clear` (`self.Path`))
  (if (`KismetSystemLibrary.IsServer`)
    (`self.GetPath` _targetlocation)
    (else
      (`self.Svr_getPath` _targetlocation))))

(event `WaypointTimer`
  (bind (_updatewaypoint _removewaypoint) (`self.CheckUpdateDistance`))
  (if _updatewaypoint
    (`self.CreateWaypoint` (`self.GoalDistance`) (`self.TargetLocation`) (`self.UpdateInterval`) (`self.Z_Offset`) (`self.UpdateDistance`) (`self.SplineLifetime`))
    (elif _removewaypoint
      (goto _label_2))))

(event `OwnerResetDelay`
  (goto _label))

(fn `CheckUpdateDistance`
  (returns (UpdateWaypoint :type Boolean) (RemoveWaypoint :type Boolean))
  (locals (Lcl_PlayerLocation :type "Vector Structure" :default (0.0 0.0 0.0)))
  (bind _goaldistance (`self.GoalDistance`))
  (bind _updatedistance (`self.UpdateDistance`))
  (set `local.Lcl_PlayerLocation` (`Actor.K2_GetActorLocation` (`self.GetOwner`)))
  (if (< (`KismetMathLibrary.Vector_DistanceSquared` (`self.TargetLocation`) (`local.Lcl_PlayerLocation`)) (* _goaldistance _goaldistance))
    (return false true)
    (elif (> (`KismetMathLibrary.Vector_DistanceSquared` (`self.WaypointStartLocation`) (`local.Lcl_PlayerLocation`)) (* _updatedistance _updatedistance))
      (return true false)
      (else
        (return false false)))))