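; Game mode for an interactive navigation map that lets the player select a start and end room.
; BeginPlay adds the room display widget to the viewport and spawns an invisible pawn at a fixed location.
; RoomClicked fills the start room, then the end room, then clears both on a further click, refreshing the display each time.
; Once both rooms are set, the pawn draws a line between their stored locations.
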(event `self.ReceiveBeginPlay`
  (bind _returnvalue (`|CreateWidget` "/Game/Navigation/InteractiveMap_2/BP_RoomDisplayUI.BP_RoomDisplayUI_C" (`GameplayStatics.GetPlayerController` 0)))
  (bind _output_get (set `self.Room Display` _returnvalue))
  (`UserWidget.AddToViewport` _output_get 0)
  (bind _returnvalue_2 (`|SpawnActorFromClass` "/Game/Navigation/InteractiveMap_2/BP_InvisPawn.BP_InvisPawn_C" (`KismetMathLibrary.MakeTransform` (-10170.0 -1970.0 230.0)) "AlwaysSpawn" "MultiplyWithRoot" null null))
  (set `self.Invis Pawn` _returnvalue_2))

(fn `Get Rooms`
  (returns (`Start Room` :type Text) (`End Room` :type Text))
  (return (`self.Start Room`) (`self.End Room`)))

(fn `RoomClicked`
  (params (Room :type Text) (Location :type "Vector Structure"))
  (if (`KismetTextLibrary.EqualEqual_TextText` (`self.Start Room`) "")
    (set `self.Start Room` (`local.Room`))
    (`self.Update Display`)
    (set `self.Start Room Location` (`local.Location`))
    (elif (`KismetTextLibrary.EqualEqual_TextText` (`self.End Room`) "")
      (set `self.End Room` (`local.Room`))
      (`self.Update Display`)
      (set `self.End Room Location` (`local.Location`))
      (`/Game/Navigation/InteractiveMap_2/BP_InvisPawn.CreateLine` (`self.Invis Pawn`) (`self.Start Room Location`) (`self.End Room Location`))
      (else
        (set `self.Start Room` "")
        (set `self.End Room` "")
        (`self.Update Display`)
        (set `self.Start Room Location` (0.0 0.0 0.0))
        (set `self.End Room Location` (0.0 0.0 0.0))))))

(fn `Update Display`
  (`/Game/Navigation/InteractiveMap_2/BP_RoomDisplayUI.Set Room Displays` (`self.Room Display`) (`self.Start Room`) (`self.End Room`)))

(fn `UserConstructionScript`)