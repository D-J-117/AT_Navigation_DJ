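; BP_SelectableRoom is a clickable room actor for the interactive navigation map, taking its room identifier from its TextRender text.
; On BeginPlay it sets its Cube to an unlit grey material and caches the map game instance.
; Cursor hover applies an overlay material, ending on M_Hologram, and unhover clears it.
; Clicking passes the room and its Entrance location to the game instance's RoomClicked.
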(event `self.ReceiveBeginPlay`
  (`PrimitiveComponent.SetMaterial` (`self.Cube`) 0 "/Game/Materials/MI_GreyUnlit.MI_GreyUnlit")
  (set `self.Default Material` (`PrimitiveComponent.GetMaterial` (`self.Cube`) 0))
  (set `self.Room` (`TextRenderComponent.Text` (`self.TextRender`)))
  (bind _asinst_map_game_instance (cast `/Game/FirstPerson/Blueprints/Inst_MapGameInstance` (`GameplayStatics.GetGameInstance`)))
  (set `self.As Inst Map Game Instance` _asinst_map_game_instance))

(event `self.Cube.OnBeginCursorOver`
  (params (TouchedComponent :type "PrimitiveComponent Object Reference"))
  (`self.Hovered`))

(event `self.Cube.OnEndCursorOver`
  (params (TouchedComponent :type "PrimitiveComponent Object Reference"))
  (`self.Unhovered`))

(event `Hovered`
  (`MeshComponent.SetOverlayMaterial` (`self.Cube`) "/Game/Materials/MI_WhiteHighlight.MI_WhiteHighlight")
  (`MeshComponent.SetOverlayMaterial` (`self.Cube`) "/Game/Materials/M_Hologram.M_Hologram"))

(event `Unhovered`
  (`MeshComponent.SetOverlayMaterial` (`self.Cube`) null))

(event `self.ReceiveActorOnClicked`
  (params (ButtonPressed :type "Key Structure"))
  (`/Game/FirstPerson/Blueprints/Inst_MapGameInstance.RoomClicked` (`self.As Inst Map Game Instance`) (`self.Room`) (`self.K2_GetActorLocation` (`self.Entrance`))))

(fn `UserConstructionScript`)